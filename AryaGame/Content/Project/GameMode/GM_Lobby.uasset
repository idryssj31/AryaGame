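; Lobby GameMode that gathers connecting players and sends the server to the test level once the session is full.
; PostLogin adds each controller to a list and compares its length to the session's connection count from GetSessionSettings.
; On a match it waits briefly, then runs a serverTravel console command to Lvl_GameTestV0.
; Logout removes the leaving controller from the list.
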(event `self.K2_PostLogin`
  (params (NewPlayer :type "PlayerController Object Reference"))
  ;[1 1 1] On player log on the session
  (`KismetArrayLibrary.Array_AddUnique` (`self.Controllers`) NewPlayer)
  (bind _numconnections (`AdvancedSessionsLibrary.GetSessionSettings`)
    (:`OnSuccess`
      (if (== _numconnections (`KismetArrayLibrary.Array_Length` (`self.Controllers`)))
        (`KismetSystemLibrary.Delay` 3.0)
        (`KismetSystemLibrary.ExecuteConsoleCommand` "serverTravel Lvl_GameTestV0" null)))))

(event `self.K2_OnLogout`
  (params (ExitingController :type "Controller Object Reference"))
  ;[1 1 1] On player outlog of the session
  (bind _asplayer_controller (cast `PlayerController` ExitingController))
  (`KismetArrayLibrary.Array_RemoveItem` (`self.Controllers`) _asplayer_controller))

(fn `UserConstructionScript`)